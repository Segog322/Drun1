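; Bait interactable actor that shows an on-screen prompt widget while the first-person player stands near it.
; Box overlap creates the InteractrBAIT widget and adds it to the viewport, and end overlap removes it.
; The Interact1 event only removes the widget; a sound spawn node at the actor's location is left unconnected and never runs.
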(event `/Game/AI/BP_OPENDOOR/BAIT_INTERACT.Interact_1`
  (`Widget.RemoveFromParent` (`self.NewVar_0`)))

(event `self.Box.OnComponentBeginOverlap`
  (params (OverlappedComponent :type "PrimitiveComponent Object Reference") (OtherActor :type "Actor Object Reference") (OtherComp :type "PrimitiveComponent Object Reference") (OtherBodyIndex :type Integer) (bFromSweep :type Boolean) (SweepResult :type "HitResult Structure (by ref)"))
  (cast `/Game/FirstPerson/Blueprints/BP_FirstPersonCharacter` OtherActor)
  (bind _returnvalue (`|CreateWidget` "/Game/AI/BP_OPENDOOR/InteractrBAIT.InteractrBAIT_C"))
  (bind _output_get (set `self.NewVar_0` _returnvalue))
  (`UserWidget.AddToViewport` _output_get 0))

(event `self.Box.OnComponentEndOverlap`
  (params (OverlappedComponent :type "PrimitiveComponent Object Reference") (OtherActor :type "Actor Object Reference") (OtherComp :type "PrimitiveComponent Object Reference") (OtherBodyIndex :type Integer))
  (cast `/Game/FirstPerson/Blueprints/BP_FirstPersonCharacter` OtherActor)
  (`Widget.RemoveFromParent` (`self.NewVar_0`)))

(fn `UserConstructionScript`)