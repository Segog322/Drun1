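; BP_BUTTONON is a Blueprint that toggles a cage on a referenced enemy when Z is pressed.
; It enables player 0 input on BeginPlay to receive the key directly.
; Without a valid Box, it spawns BP_CUBEDESTROY at EnemyRef's location, stores it as Box and disables the enemy's movement.
; With a valid Box, it destroys that actor and restores the enemy's Walking mode.
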(event `self.ReceiveBeginPlay`
  ; Клетка
  (`self.EnableInput` (`GameplayStatics.GetPlayerController` 0)))

(event `Key|Z`
  (params (Key :type "Key Structure"))
  ; Клетка
  (:`Pressed`
    (`/Engine/EditorBlueprintResources/StandardMacros.IsValid` (`self.Box`)
      (:`Is Valid`
        (`self.K2_DestroyActor` (`self.Box`))
        (`CharacterMovementComponent.SetMovementMode` (`Character.CharacterMovement` (`self.EnemyRef`)) "MOVE_Walking" 0))
      (:`Is Not Valid`
        (bind _returnvalue (`|SpawnActorFromClass` "/Game/Blueprints/BP_CUBEDESTROY.BP_CUBEDESTROY_C" (`KismetMathLibrary.MakeTransform` (`self.K2_GetActorLocation` (`self.EnemyRef`))) "AlwaysSpawn" "MultiplyWithRoot" null null))
        (set `self.Box` _returnvalue)
        (`CharacterMovementComponent.DisableMovement` (`Character.CharacterMovement` (`self.EnemyRef`)))))))

(fn `UserConstructionScript`)